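; BP_HH randomly assigns the Hunter role to a BP_Character and shows every character's role as debug text.
; On BeginPlay it gathers all BP_Character actors and sets Hunter on one at a random index from 1 to the last, so the first is never picked.
; Each Tick it gathers them again and prints each display name with its Hunter flag.
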(event `self.ReceiveTick`
  (params (DeltaSeconds :type "Float (single-precision)"))
  (bind _outactors (`GameplayStatics.GetAllActorsOfClass` "/Game/Blueprints/Characters/BP_Character.BP_Character_C"))
  (for _array_element _outactors
    (`/Game/Blueprints/Game/BP_CustomFunctionLibrary.MyPrintText` (`KismetTextLibrary.Conv_TextToString` (`|FormatText` "Name {A}    Hunter? {B}" (`KismetSystemLibrary.GetDisplayName` _array_element) (`/Game/Blueprints/Characters/BP_Character.Hunter?` _array_element))) (struct :`R` 0.619792 :`G` 0.037727 :`A` 1.0) 0.0)))

(event `self.ReceiveBeginPlay`
  (bind _outactors (`GameplayStatics.GetAllActorsOfClass` "/Game/Blueprints/Characters/BP_Character.BP_Character_C"))
  (set `/Game/Blueprints/Characters/BP_Character.Hunter?` true (`|GetArrayItem` _outactors (`KismetMathLibrary.RandomIntegerInRange` 1 (`KismetArrayLibrary.Array_LastIndex` _outactors)))))

(fn `UserConstructionScript`)