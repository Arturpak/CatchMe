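; BP_Ai is an AI character Blueprint, derived from a parent class, that carries a BPAmplifier for spell-based boosters.
; Its construction script runs the parent's script, then copies its Stars value into the amplifier.
; PrintTextDebug prints the name, security mode, stars and current booster.
; Tick and BeginPlay are empty; delayed spell casting and Hunter-based mesh visibility exist only as unconnected nodes.
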(event `self.ReceiveTick`
  (params (DeltaSeconds :type "Float (single-precision)")))

(event `self.ReceiveBeginPlay`)

(fn `PrintTextDebug`
  (`KismetSystemLibrary.PrintString` (`KismetTextLibrary.Conv_TextToString` (`|FormatText` "-------------------------------- \nName - {E} \nSecurity Mode {C} \nStar {D} \nИмеется бустер?   {F} \n--------------------------------" (`self.Name`) (`/Game/Blueprints/Game/Pickup/BP_Amplifier.SecurityMode` (`self.BP_Amplifier`)) (`/Game/Blueprints/Game/Pickup/BP_Amplifier.Stars` (`self.BP_Amplifier`)) (select `bool` (`/Game/Blueprints/Game/Pickup/BP_Amplifier.IsThere? ` (`self.BP_Amplifier`)) :`false` (`|FormatText` "No") :`true` (`.Name_5_48EAE1FD4DE63B28DAC50ABD6BB61368` (break `/Game/Blueprints/Game/Pickup/Data/S_Amplifier` (`/Game/Blueprints/Game/Pickup/BP_Amplifier.Current` (`self.BP_Amplifier`))))))) true true (struct :`G` 0.66 :`B` 1.0 :`A` 1.0) 0.0))

(fn `UserConstructionScript`
  (`parent.UserConstructionScript`)
  (set `/Game/Blueprints/Game/Pickup/BP_Amplifier.Stars` (`self.Stars`) (`self.BP_Amplifier`)))