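; Main menu HUD Blueprint that shows and hides the W_MainMenu widget, displaying it on BeginPlay.
; Showing creates and caches the widget if needed, adds it to the viewport, sets UI-only input focused on it and enables the mouse cursor for player 0.
; Hiding removes the widget, clears the cached reference and turns the cursor off, but leaves the input mode unchanged.
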(event `self.ReceiveBeginPlay`
  (`self.DisplayHUD_MainMenu` true))

(event `DisplayHUD_MainMenu`
  (params (Condition :type Boolean))
  (if Condition
    (`self.W_HUD_MainMenu`
      (:`then`
        _)
      (:`else`
        (bind _returnvalue (`|CreateWidget` "/Game/Blueprints/Game/Interface/MainMenu/W_MainMenu.W_MainMenu_C" (`GameplayStatics.GetPlayerController` 0)))
        (bind _output_get (set `self.W_HUD_MainMenu` _returnvalue))))
    (`UserWidget.AddToViewport` _output_get 0)
    (`WidgetBlueprintLibrary.SetInputMode_UIOnlyEx` (`GameplayStatics.GetPlayerController` 0) _output_get)
    (set `PlayerController.bShowMouseCursor` true (`GameplayStatics.GetPlayerController` 0))
    (else
      (bind _w_hud_mainmenu (`self.W_HUD_MainMenu`)
        (:`then`
          (`Widget.RemoveFromParent` _w_hud_mainmenu)
          (set `self.W_HUD_MainMenu` null)
          (set `PlayerController.bShowMouseCursor` false (`GameplayStatics.GetPlayerController` 0)))
        (:`else`)))))

(fn `UserConstructionScript`)