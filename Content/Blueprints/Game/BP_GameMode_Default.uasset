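; Default game mode that runs a timed round from pre-round screen to results.
; BeginPlay copies the player's name from the game instance, disables character input and shows the pre-round widget, then the HUD after its delay.
; A looping one-second timer counts down minutes and seconds once the Start flag is set.
; When the end check passes, it flags Finish, shows results and clears the timer; Tick then keeps input disabled.
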(event Custom|Start
  (if (Variables|/Game/Blueprints/Game/BP_GameInstance.BP_GameInstance_C|GetStart? (CallFunction|MyGameInstance))
    (CallFunction|SetTimer)
    (if (|(({A7FB80C2-4D03-E146-460C-BDB79BBBF53E}==0)&&({987C97AB-4FAB-D669-2AEA-94BFD4B6DFAF}==0)))
      (Variables|/Game/Blueprints/Game/BP_GameInstance.BP_GameInstance_C|SetFinish? (CallFunction|MyGameInstance) true)
      (Widget|SetVisibility (Variables|/Game/Blueprints/Game/Interface/HUD/W_HUD.W_HUD_C|GetCanvasPanelDefault (Variables|/Game/Blueprints/Game/BP_HUD.BP_HUD_C|GetW_HUD (CallFunction|MyHUD))) "Hidden")
      (Default|DisplayResultWidget (CallFunction|MyHUD) true)
      (Default|ResultNodePlay (Variables|/Game/Blueprints/Game/BP_HUD.BP_HUD_C|GetW_Result (CallFunction|MyHUD)))
      (Utilities|Time|ClearandInvalidateTimerbyHandle (Variables|Default|GetTimer)))))

(event EventBeginPlay
  (bind _hud (CallFunction|MyHUD))
  (Variables|/Game/Blueprints/Characters/BP_Character.BP_Character_C|SetName (CallFunction|MyPlayer) (Variables|/Game/Blueprints/Game/BP_GameInstance.BP_GameInstance_C|GetName (CallFunction|MyGameInstance)))
  (bind _returnvalue (Utilities|Time|SetTimerbyEvent (delegate Custom|Start) 1.0 true))
  (Variables|Default|SetTimer _returnvalue)
  (Default|InpitCharacters _hud false)
  (Default|DisplayPreRoundWidget _hud true)
  (Utilities|FlowControl|Delay (Math|Conversions|ToFloat(Integer) (Variables|/Game/Blueprints/Game/Interface/W_PreRound.W_PreRound_C|GetSeconds (Variables|/Game/Blueprints/Game/BP_HUD.BP_HUD_C|GetW_PreRound (CallFunction|MyHUD)))))
  (Default|DisplayHUD (CallFunction|MyHUD) true))

(event EventTick
  (params (DeltaSeconds :type Float%20%28single-precision%29))
  (if (Variables|/Game/Blueprints/Game/BP_GameInstance.BP_GameInstance_C|GetFinish? (CallFunction|MyGameInstance))
    (Default|InpitCharacters (CallFunction|MyHUD) false)))

(fn ConstructionScript
  (|CallParentFunction))

(fn SetTimer
  (if (== (Variables|Default|GetSeconds) 0)
    (if (not (== (Variables|Default|GetMinutes) 0))
      (Variables|Default|SetSeconds 59)
      (Variables|Default|SetMinutes (- (Variables|Default|GetMinutes) 1))
      (return))
    (else
      (Variables|Default|SetSeconds (- (Variables|Default|GetSeconds) 1))
      (return))))