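; BP_Amplifier is a pickup amplifier that applies a timed Speed, Jump or Security Mode effect to a character.
; ApplySpell runs only while IsThere is set, then switches on the type, using values from Current.
; Speed also plays audio; Speed and Jump reset to hard-coded defaults after a delay, while Security Mode is never reverted here.
; Each effect ends by clearing Active and blanking the HUD's amplifier icon and name.
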(event `ApplySpell`
  (params (Character :type "/Game/Blueprints/Characters/BP_Character Object Reference"))
  (bind _audio (`/Game/Blueprints/Characters/BP_Character.Audio` (`self.Character`)))
  (set `self.Character` Character)
  (if (`self.IsThere? `)
    (set `self.Active?` true)
    (switch `/Game/Blueprints/Game/Pickup/Data/E_Amplifier` (`self.Amplifier`)
      (:`NewEnumerator0`
        (set `self.IsThere? ` false)
        ;[0.03646 0.03646 0.03646] + Speed
        (set `CharacterMovementComponent.MaxWalkSpeed` (+ (`.Movement_15_40742500434F651C9B1640B35E8C4105` (break `/Game/Blueprints/Game/Pickup/Data/S_Amplifier` (`self.Current`))) (`CharacterMovementComponent.MaxWalkSpeed` (`Character.CharacterMovement` (`self.Character`)))) (`Character.CharacterMovement` (`self.Character`)))
        (`AudioComponent.SetSound` _audio (`.Sound_22_53D690864FC1994C665B01A60934F62E` (break `/Game/Blueprints/Game/Pickup/Data/S_Amplifier` (`self.Current`))))
        (`AudioComponent.FadeIn` _audio 0.0 1.0 4.0 "Linear")
        (`KismetSystemLibrary.Delay` 5.0)
        (set `CharacterMovementComponent.MaxWalkSpeed` 650.0 (`Character.CharacterMovement` (`self.Character`))))
      (:`NewEnumerator1`
        (set `self.IsThere? ` false)
        (set `CharacterMovementComponent.JumpZVelocity` (+ (`CharacterMovementComponent.JumpZVelocity` (`Character.CharacterMovement` (`self.Character`))) (`.Movement_15_40742500434F651C9B1640B35E8C4105` (break `/Game/Blueprints/Game/Pickup/Data/S_Amplifier` (`self.Current`)))) (`Character.CharacterMovement` (`self.Character`)))
        (`KismetSystemLibrary.Delay` 10.0)
        (set `CharacterMovementComponent.JumpZVelocity` 370.0 (`Character.CharacterMovement` (`self.Character`))))
      (:`NewEnumerator2`
        (set `self.IsThere? ` false)
        (bind _output_get (set `self.SecurityMode` (`.SecurityMode_16_CE4FA80F42B032912339CDBFF44987F0` (break `/Game/Blueprints/Game/Pickup/Data/S_Amplifier` (`self.Current`)))))
        (set `/Game/Blueprints/Characters/BP_Character.SecurityMode` _output_get (`self.Character`))
        (`KismetSystemLibrary.Delay` 10.0)))
    (set `self.Active?` false)
    (`self.SetBrushClear`)))

(fn `SetBrushClear`
  (bind _w_hud (`/Game/Blueprints/Game/BP_HUD.W_HUD` (`/Game/Blueprints/Game/BP_CustomFunctionLibrary.MyHUD`)))
  (`Border.SetBrush` (`/Game/Blueprints/Game/Interface/HUD/W_HUD.I_Amplifier` _w_hud) (make `SlateBrush` :`TintColor` (make `SlateColor` (struct :`R` 1.0 :`G` 1.0 :`B` 1.0))))
  (`TextBlock.SetText` (`/Game/Blueprints/Game/Interface/HUD/W_HUD.T_NameAmplifier` _w_hud) ""))