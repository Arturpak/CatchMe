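; Pickup platform that grants an overlapping BP_Character a Speed, Jump, Security Mode or Star amplifier, fixed or random.
; Rows from DT_Amplifier fill the character's BPAmplifier and update the local player's HUD, while Stars add to a count.
; A held amplifier blocks new grants, and an active one allows only a configured Star.
; After a grant the platform reloads, with a dynamic material turning red on overlaps during cooldown.
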(event `self.ReceiveBeginPlay`
  (bind _returnvalue (`PrimitiveComponent.CreateDynamicMaterialInstance` (`self.StaticMesh`) 0 "/Game/Assets/Materials/GridMaterial/M_GridCustom_Inst5.M_GridCustom_Inst5" "Color"))
  (set `self.MatInstance` _returnvalue))

(event `self.Box.OnComponentBeginOverlap`
  (params (OverlappedComponent :type "PrimitiveComponent Object Reference") (OtherActor :type "Actor Object Reference") (OtherComp :type "PrimitiveComponent Object Reference") (OtherBodyIndex :type Integer) (bFromSweep :type Boolean) (SweepResult :type "HitResult Structure (by ref)"))
  (if (`self.ActivePlatform?`)
    (bind _asbp_character (cast `/Game/Blueprints/Characters/BP_Character` OtherActor))
    (bind _output_get (set `self.BP Character` _asbp_character))
    (if (`/Game/Blueprints/Game/Pickup/BP_Amplifier.Active?` (`/Game/Blueprints/Characters/BP_Character.BP_Amplifier` _output_get))
      (if (`|EnumEquality` (`self.Amplifier`) "NewEnumerator3")
        (`self.SetAmplifierStar`)
        (set `self.ActivePlatform?` false)
        (`KismetSystemLibrary.Delay` (`self.Reloading`))
        (set `self.ActivePlatform?` true))
      (elif (not (`/Game/Blueprints/Game/Pickup/BP_Amplifier.IsThere? ` (`/Game/Blueprints/Characters/BP_Character.BP_Amplifier` (`self.BP Character`))))
        (if (`self.Random?`)
          ;[0.05208 0.05208 0.05208] Random
          (switch `/Game/Blueprints/Game/Pickup/Data/E_Amplifier` (cast `/Game/Blueprints/Game/Pickup/Data/E_Amplifier` (`KismetMathLibrary.Conv_IntToByte` (`KismetMathLibrary.RandomIntegerInRange` 0 3)))
            (:`NewEnumerator0`
              (`self.SetAmplifier` "Speed"))
            (:`NewEnumerator1`
              (`self.SetAmplifier` "Jump" "NewEnumerator1"))
            (:`NewEnumerator2`
              (`self.SetAmplifier` "SecurityMode" "NewEnumerator2"))
            (:`NewEnumerator3`
              (set `self.Star?` true)
              (`self.SetAmplifierStar`)))
          (else
            ;[0.05208 0.05208 0.05208] Comment
            (switch `/Game/Blueprints/Game/Pickup/Data/E_Amplifier` (`self.Amplifier`)
              (:`NewEnumerator0`
                (`self.SetAmplifier` "Speed" (`self.Amplifier`)))
              (:`NewEnumerator1`
                (`self.SetAmplifier` "Jump" (`self.Amplifier`)))
              (:`NewEnumerator2`
                (`self.SetAmplifier` "SecurityMode" (`self.Amplifier`)))
              (:`NewEnumerator3`
                (`self.SetAmplifierStar`)))))
        (set `self.ActivePlatform?` false)
        (`KismetSystemLibrary.Delay` (`self.Reloading`))
        (set `self.ActivePlatform?` true)
        (`KismetSystemLibrary.PrintString` "Активнв")
        (`MaterialInstanceDynamic.SetVectorParameterValue` (`self.MatInstance`) "Color" (struct :`R` 1.0 :`G` 0.89627 :`A` 1.0))))
    (else
      (`MaterialInstanceDynamic.SetVectorParameterValue` (`self.MatInstance`) "Color" (struct :`R` 1.0 :`B` 0.018451 :`A` 1.0)))))

(fn `SetAmplifier`
  (params (RowName :type Name) (Amplifier :type "/Game/Blueprints/Game/Pickup/Data/E_Amplifier Enum" :default "NewEnumerator0"))
  (locals (L_CurrentBuster :type "/Game/Blueprints/Game/Pickup/Data/S_Amplifier Structure"))
  (bind _bp_amplifier (`/Game/Blueprints/Characters/BP_Character.BP_Amplifier` (`self.BP Character`)))
  (bind _returnvalue (`|GetDataTableRow` "/Game/Blueprints/Game/Pickup/Data/DT_Amplifier.DT_Amplifier" RowName)
    (:`then`
      (bind _output_get (set `local.L_CurrentBuster` _returnvalue))
      (set `/Game/Blueprints/Game/Pickup/BP_Amplifier.Current` _output_get _bp_amplifier)
      (set `/Game/Blueprints/Game/Pickup/BP_Amplifier.Amplifier` Amplifier _bp_amplifier)
      (set `/Game/Blueprints/Game/Pickup/BP_Amplifier.IsThere? ` true _bp_amplifier)
      (if (== (`/Game/Blueprints/Game/BP_CustomFunctionLibrary.MyPlayer`) (`self.BP Character`))
        (`self.SetBrush` (`local.L_CurrentBuster`))))))

(fn `SetAmplifierStar`
  (bind _returnvalue (`|GetDataTableRow` "/Game/Blueprints/Game/Pickup/Data/DT_Amplifier.DT_Amplifier" "Star")
    (:`then`
      (set `/Game/Blueprints/Game/Pickup/BP_Amplifier.Stars` (+ (`.Star_11_59670B5444094785DAB68382C0A8AC4A` (break `/Game/Blueprints/Game/Pickup/Data/S_Amplifier` _returnvalue)) (`/Game/Blueprints/Game/Pickup/BP_Amplifier.Stars` (`/Game/Blueprints/Characters/BP_Character.BP_Amplifier` (`self.BP Character`)))) (`/Game/Blueprints/Characters/BP_Character.BP_Amplifier` (`self.BP Character`)))
      (return))))

(fn `SetBrush`
  (params (NewParam :type "/Game/Blueprints/Game/Pickup/Data/S_Amplifier Structure"))
  (bind ((`Name_5_48EAE1FD4DE63B28DAC50ABD6BB61368` _name) (`Icon_19_28F5592F4ED7EEDFEB55ACBFFCAC2195` _icon)) (break `/Game/Blueprints/Game/Pickup/Data/S_Amplifier` NewParam))
  (bind _w_hud (`/Game/Blueprints/Game/BP_HUD.W_HUD` (`/Game/Blueprints/Game/BP_CustomFunctionLibrary.MyHUD`)))
  (`Border.SetBrush` (`/Game/Blueprints/Game/Interface/HUD/W_HUD.I_Amplifier` _w_hud) (make `SlateBrush` :`ResourceObject` _icon))
  (`TextBlock.SetText` (`/Game/Blueprints/Game/Interface/HUD/W_HUD.T_NameAmplifier` _w_hud) _name))

(fn `UserConstructionScript`)