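; BP_CustomFunctionLibrary is a helper library of shortcuts to the game's core objects plus a debug print.
; Its getters cast the first player's HUD, the player character and the game instance to project Blueprint classes.
; MyPlayer, MyAiCharacter and MyCharacterAll all cast player character 0, so the AI getter never searches for other characters.
; MyPrintText wraps PrintString with text, color and duration inputs.
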(fn `MyAiCharacter`
  (returns (`Ai Character` :type "/Game/Blueprints/Characters/BP_Ai Object Reference"))
  (bind _asbp_ai (cast `/Game/Blueprints/Characters/BP_Ai` (`GameplayStatics.GetPlayerCharacter` null)))
  (return _asbp_ai))

(fn `MyCharacterAll`
  (returns (Character :type "/Game/Blueprints/Characters/BP_Character Object Reference"))
  (bind _asbp_character (cast `/Game/Blueprints/Characters/BP_Character` (`GameplayStatics.GetPlayerCharacter` null)))
  (return _asbp_character))

(fn `MyGameInstance`
  (returns (`Game Instance` :type "/Game/Blueprints/Game/BP_GameInstance Object Reference"))
  (bind _asbp_game_instance (cast `/Game/Blueprints/Game/BP_GameInstance` (`GameplayStatics.GetGameInstance` null)))
  (return _asbp_game_instance))

(fn `MyHUD`
  (returns (HUD :type "/Game/Blueprints/Game/BP_HUD Object Reference"))
  (bind _asbp_hud (cast `/Game/Blueprints/Game/BP_HUD` (`PlayerController.GetHUD` (`GameplayStatics.GetPlayerController` null))))
  (return _asbp_hud))

(fn `MyPlayer`
  (returns (`My Player` :type "/Game/Blueprints/Characters/BP_Player Object Reference"))
  (bind _asbp_player (cast `/Game/Blueprints/Characters/BP_Player` (`GameplayStatics.GetPlayerCharacter` null)))
  (return _asbp_player))

(fn `MyPrintText`
  (params (Text :type String :default "Text") (Color :type "LinearColor Structure" :default (struct :`R` 0.437468 :`G` 0.619792 :`B` 0.205791 :`A` 1.0)) (Duration :type "Float (double-precision)" :default 3.0))
  (`KismetSystemLibrary.PrintString` null Text true true Color Duration))